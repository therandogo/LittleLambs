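; Interactive book actor whose pages are turned by dragging with the mouse.
; When the player enters its box, the view blends to the book, character input is disabled, and the cursor and book input are enabled.
; IA_PageTurn line-traces under the cursor to grab a component, then converts horizontal mouse offset into world pitch.
; The clamp range depends on press X versus the last recorded release X.
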(event OnComponentBeginOverlap(Box)
  (params (OverlappedComponent :type Primitive%20Component%20Object%20Reference) (OtherActor :type Actor%20Object%20Reference) (OtherComp :type Primitive%20Component%20Object%20Reference) (OtherBodyIndex :type Integer) (bFromSweep :type Boolean) (SweepResult :type Hit%20Result%20Structure%20%28by%20ref%29))
  (bind _returnvalue (Game|GetPlayerController 0))
  (bind _returnvalue_2 (Game|GetPlayerCharacter 0))
  (if (== OtherActor _returnvalue_2)
    (Game|Player|SetViewTargetwithBlend _returnvalue self 0.0 "VTBlend_Linear" 0.0 false)
    (Input|DisableInput _returnvalue_2 _returnvalue)
    (Variables|/Script/Engine.PlayerController|SetbShowMouseCursor _returnvalue true)
    (Input|EnableInput (Game|GetPlayerController 0))))

(event Input|EnhancedActionEvents|EnhancedInputActionIA_PageTurn
  (params (ActionValue :type Float%20%28double-precision%29) (ElapsedSeconds :type Float%20%28double-precision%29) (TriggeredSeconds :type Float%20%28double-precision%29) (InputAction :type Input%20Action%20Object%20Reference :default "/Game/FirstPerson/Input/Actions/IA_PageTurn.IA_PageTurn"))
  (bind _returnvalue (Game|GetPlayerController 0))
  (bind _returnvalue_2 (Game|GetPlayerController 0))
  (bind (_worldlocation _worlddirection) (Game|Player|ConvertMouseLocationToWorldSpace _returnvalue))
  (bind _locationx (Game|Player|GetMousePosition _returnvalue_2))
  (:Triggered
    (Variables|Default|SetCurrentMouseX (.LocationX (Game|Player|GetMousePosition (Game|GetPlayerController 0))))
    (bind _output_get (Variables|Default|SetDelta (- (Variables|Default|GetCurrentMouseX) (Variables|Default|GetInitialMouseX))))
    (bind _output_get_2 (Variables|Default|SetTargetRotation (select (> (Variables|Default|GetPrevious%20X%20Location) (Variables|Default|GetLocation%20X)) (Math|Float|Clamp(Float) (- (Variables|Default|GetTargetRotation) (* _output_get 0.01)) 1.8e+02 3.6e+02) (Math|Float|Clamp(Float) (- (Variables|Default|GetTargetRotation) (* _output_get 0.01)) -1.8e+02 0.0))))
    (bind _hit_component (Variables|Default|GetHit%20Component)
      (:then
        (Transformation|SetWorldRotation _hit_component (Math|Rotator|MakeRotator 0.0 _output_get_2 0.0) false false))
      (:else)))
  (:Started
    (Variables|Default|SetIsPageHeld? true)
    (bind (_outhit _returnvalue_3) (Collision|LineTraceByChannel _worldlocation (+ _worldlocation (* _worlddirection 5e+03)) "TraceTypeQuery1" false (Utilities|Array|MakeArray (Game|GetPlayerCharacter 0)) "None" false))
    (if _returnvalue_3
      (Variables|Default|SetHit%20Component (.HitComponent (Collision|BreakHitResult _outhit)))
      (bind _hit_component_2 (Variables|Default|GetHit%20Component)
        (:then
          (if (Utilities|Enum|Equal(Enum) (Variables|/Script/Engine.SceneComponent|GetMobility _hit_component_2) "Movable")
            (Variables|Default|SetInitialMouseX _locationx)
            (Variables|Default|SetPrevious%20X%20Location _locationx)))
        (:else))))
  (:Completed
    (Variables|Default|SetIsPageHeld? false)
    (Variables|Default|SetLocation%20X (.LocationX (Game|Player|GetMousePosition (Game|GetPlayerController 0))))))

(event EventBeginPlay)

(fn ConstructionScript)