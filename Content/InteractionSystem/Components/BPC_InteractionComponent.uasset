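; Actor component that lets its owning character hover, interact with, hold, drop and inspect actors carrying a BPC_InteractableComponent.
; A looping timer line-traces from the owner's camera to track focus; interacting passes the physics handle and camera to the interactable and applies its walking speed until drop.
; A faster timer checks the movement floor, sending stood-on/off messages and allowing new interactions only while grounded.
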(event Custom|InteractWithFocusedActor
  (CallFunction|Interact))

(event EventBeginPlay
  (CallFunction|SetOwnerAttributes)
  (Utilities|Time|SetTimerbyFunctionName 0 "Raycast" 0.1 true)
  (Utilities|Time|SetTimerbyFunctionName 0 "StandOnInteractableCheck" 0.01 true))

(fn Raycast
  (bind _ownercamera (Variables|Default|GetOwnerCamera))
  (bind _returnvalue (Transformation|GetWorldLocation _ownercamera))
  (bind (_outhit _returnvalue_2) (Collision|LineTraceByChannel _returnvalue (+ _returnvalue (* (Math|Vector|GetForwardVector _ownercamera) (Variables|InteractionSettings|GetInteractDistance))) "TraceTypeQuery1" false 0 "None"))
  (if _returnvalue_2
    (if (!= (Variables|FocusedActor|GetInFocusActor) (.HitActor (Collision|BreakHitResult _outhit)))
      (bind _bpc_interacatable (Variables|Default|GetBPC_Interacatable)
        (:then
          (Class|BPIInteraction|HoveredCheck(Message) _bpc_interacatable false))
        (:else
          _))
      (Variables|FocusedActor|SetInFocusActor (.HitActor (Collision|BreakHitResult _outhit)))
      (Utilities|IsValid (Actor|GetComponentbyClass (.HitActor (Collision|BreakHitResult _outhit)) "/Game/InteractionSystem/Components/BPC_InteractableComponent.BPC_InteractableComponent_C")
        (:Is%20Valid
          (Class|BPIInteraction|HoveredCheck(Message) (Actor|GetComponentbyClass (.HitActor (Collision|BreakHitResult _outhit)) "/Game/InteractionSystem/Components/BPC_InteractableComponent.BPC_InteractableComponent_C") true)
          (Variables|Default|SetBPC_Interacatable (Actor|GetComponentbyClass (.HitActor (Collision|BreakHitResult _outhit)) "/Game/InteractionSystem/Components/BPC_InteractableComponent.BPC_InteractableComponent_C")))))
    (else
      (bind _bpc_interacatable_2 (Variables|Default|GetBPC_Interacatable)
        (:then
          (Class|BPIInteraction|HoveredCheck(Message) _bpc_interacatable_2 false)
          (Variables|FocusedActor|SetInFocusActor 0)
          (Variables|Default|SetBPC_Interacatable 0))
        (:else)))))

(fn SetOwnerAttributes
  (bind _output_get (Variables|Owner|SetOwnerActor (Components|GetOwner)))
  (Variables|Default|SetOwnerCamera (Actor|GetComponentbyClass _output_get "/Script/Engine.CameraComponent"))
  (Variables|Default|SetPhysicsHandler (Actor|GetComponentbyClass (Variables|Owner|GetOwnerActor) "/Script/Engine.PhysicsHandleComponent"))
  (Variables|Default|SetCharacterMovement (Actor|GetComponentbyClass (Variables|Owner|GetOwnerActor) "/Script/Engine.CharacterMovementComponent")))

(fn Interact
  (if (Variables|InteractionSettings|GetIsHolding)
    (CallFunction|StopInteraction)
    (elif (Variables|InteractionSettings|GetCanInteract)
      (bind _bpc_interacatable (Variables|Default|GetBPC_Interacatable)
        (:then
          (if (Default|GetCanInteract _bpc_interacatable)
            (Class|BPIInteraction|OnInteract(Message) (Variables|Default|GetBPC_Interacatable) (Variables|Default|GetPhysicsHandler) (Variables|Default|GetOwnerCamera))
            (CallFunction|SetInteractionDependencies)))
        (:else)))))

(fn StopInteraction
  (Variables|FocusedActor|GetHeldActor
    (:then
      (Class|BPIInteraction|OnDrop(Message) (Variables|Default|GetInteractedComponent))
      (Variables|InteractionSettings|SetIsHolding false)
      (Variables|FocusedActor|SetHeldActor 0)
      (Variables|Default|SetInteractedComponent 0)
      (Variables|/Script/Engine.CharacterMovementComponent|SetMaxWalkSpeed (Variables|Default|GetCharacterMovement) (Variables|InteractionSettings|GetDefaultWalkingSpeed)))
    (:else)))

(fn Inspect
  (params (MouseXY :type Vector%202D%20Structure))
  (bind _bpc_interacatable (Variables|Default|GetBPC_Interacatable))
  (Class|BPIInteraction|OnInspect(Message) _bpc_interacatable MouseXY)
  (return (and (Utilities|IsValid _bpc_interacatable) (Variables|InteractionSettings|GetIsHolding))))

(fn StopInspect
  (Class|BPIInteraction|StopInspect(Message) (Variables|Default|GetBPC_Interacatable)))

(fn StandonInteractableCheck
  (bind _charactermovement (Variables|Default|GetCharacterMovement))
  (bind _currentfloor (Variables|/Script/Engine.CharacterMovementComponent|GetCurrentFloor _charactermovement))
  (bind _hitresult (Utilities|Struct|BreakFindFloorResult _currentfloor))
  (bind (_bblockinghit _binitialoverlap _time _distance _location _impactpoint _normal _impactnormal _physmat _hitactor) (Collision|BreakHitResult _hitresult))
  (bind _returnvalue (Actor|GetComponentbyClass _hitactor "/Game/InteractionSystem/Components/BPC_InteractableComponent.BPC_InteractableComponent_C"))
  (if _bblockinghit
    (if (!= (Variables|StoodOnActor|GetStoodOnObject) _hitactor)
      (CallFunction|SetCanInteractWObjects true)
      (bind _stoodonbpcinteractable (Variables|Default|GetStoodOnBPCInteractable :!label _label)
        (:then
          (Class|BPIInteraction|StoodOff(Message) _stoodonbpcinteractable)
          (Variables|StoodOnActor|SetStoodOnObject 0)
          (Variables|Default|SetStoodOnBPCInteractable 0))
        (:else
          _))
      (Utilities|IsValid _hitactor
        (:Is%20Valid
          (if (Utilities|IsValid _returnvalue)
            (Class|BPIInteraction|Stoodon(Message) _returnvalue)
            (Variables|StoodOnActor|SetStoodOnObject _hitactor)
            (Variables|Default|SetStoodOnBPCInteractable _returnvalue)))))
    (else
      (CallFunction|SetCanInteractWObjects false)
      (goto _label))))

(fn SetCanInteractWObjects
  (params (CanInteract :type Boolean))
  (Variables|InteractionSettings|SetCanInteract CanInteract))

(fn SetInteractionDependencies
  (Variables|InteractionSettings|SetIsHolding true)
  (Variables|FocusedActor|SetHeldActor (Variables|FocusedActor|GetInFocusActor))
  (Variables|Default|SetInteractedComponent (Variables|Default|GetBPC_Interacatable))
  (Variables|/Script/Engine.CharacterMovementComponent|SetMaxWalkSpeed (Variables|Default|GetCharacterMovement) (Variables|/Game/InteractionSystem/Components/BPC_InteractableComponent.BPC_InteractableComponent_C|GetWalkingSpeedValue (Variables|Default|GetBPC_Interacatable))))