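; Actor component that makes its owner's static mesh hoverable, grabbable and inspectable, with hover shown through custom depth.
; A passed-in physics handle holds the mesh ahead of the camera on Tick, adding mouse delta to rotation during inspection.
; While stood on, it blocks interaction and a looping timer traces down, freezing physics over any support.
; Stood-on and stood-off messages pass to interactable supporting actors, so stacks respond together.
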(event EventOnInteract
  (params (PhysicsHandler :type Physics%20Handle%20Component%20Object%20Reference) (CameraComponent :type Camera%20Component%20Object%20Reference))
  (if (Variables|ObjectState|GetCanInteract)
    (CallFunction|OnInteraction PhysicsHandler CameraComponent)))

(event EventTick
  (params (DeltaSeconds :type Float%20%28single-precision%29))
  (if (Variables|ObjectState|GetInInteraction)
    (CallFunction|InspectionHandlingWCamera)))

(event EventHoveredCheck
  (params (IsHovered :type Boolean))
  (CallFunction|OnHoverRenderPass IsHovered))

(event EventBeginPlay
  (CallFunction|SetOwnerAttributes))

(event EventOnDrop
  (CallFunction|OnStopInteraction))

(event EventOnInspect
  (params (MouseDelta :type Vector%202D%20Structure))
  (Variables|MouseInput|SetMouse%20Delta MouseDelta)
  (Variables|ObjectState|SetInInspection true))

(event EventStopInspect
  (Variables|ObjectState|SetInInspection false))

(event EventStoodon
  (Variables|ObjectState|SetCanInteract false)
  (Variables|SupportingActor|SetSupportingActor 0)
  (bind _returnvalue (Utilities|Time|SetTimerbyFunctionName 0 "OnStoodOn" 0.01 true)))

(event EventStoodOff
  (Variables|ObjectState|SetCanInteract true)
  (Physics|SetSimulatePhysics (Variables|Default|GetOwnerStaticMesh) true)
  (Utilities|Time|PauseTimerbyHandle (stale EventStoodon _returnvalue))
  (bind _supportingactor (Variables|SupportingActor|GetSupportingActor)
    (:then
      (Class|BPIInteraction|StoodOff(Message) (Actor|GetComponentbyClass _supportingactor "BPC_InteractableComponent_C")))
    (:else)))

(fn SetOwnerAttributes
  (bind _output_get (Variables|Owner|SetOwnerActor (Components|GetOwner)))
  (Variables|Default|SetOwnerStaticMesh (Actor|GetComponentbyClass _output_get "/Script/Engine.StaticMeshComponent")))

(fn OnHoverRenderPass
  (params (bValue :type Boolean))
  (Rendering|SetRenderCustomDepth (Variables|Default|GetOwnerStaticMesh) bValue))

(fn OnInteraction
  (params (Physics%20Handler :type Physics%20Handle%20Component%20Object%20Reference) (Camera%20Component :type Camera%20Component%20Object%20Reference))
  (bind _ownerstaticmesh (Variables|Default|GetOwnerStaticMesh))
  (bind _ownerstaticmesh_2 (Variables|Default|GetOwnerStaticMesh))
  (Variables|Default|SetPhysics%20Handler Physics%20Handler)
  (Variables|Default|SetCamera%20Component Camera%20Component)
  (Physics|Components|PhysicsHandle|GrabComponentatLocationwithRotation (Variables|Default|GetPhysics%20Handler) _ownerstaticmesh_2 "None" (Transformation|GetWorldLocation _ownerstaticmesh) (Transformation|GetWorldRotation _ownerstaticmesh))
  (if (Variables|ObjectProperty|GetCollisionOverrideInActor)
    _
    (else
      (Collision|SetCollisionResponsetoChannel _ownerstaticmesh_2 "ECC_Pawn" "ECR_Ignore")))
  (Variables|ObjectState|SetInInteraction true))

(fn OnStopInteraction
  (Physics|Components|PhysicsHandle|ReleaseComponent (Variables|Default|GetPhysics%20Handler))
  (Variables|Default|SetPhysics%20Handler 0)
  (Variables|Default|SetCamera%20Component 0)
  (if (Variables|ObjectProperty|GetCollisionOverrideInActor)
    _
    (else
      (Collision|SetCollisionResponsetoChannel (Variables|Default|GetOwnerStaticMesh) "ECC_Pawn" "ECR_Block")))
  (Variables|ObjectState|SetInInteraction false))

(fn InspectionHandlingWCamera
  (bind _camera_component (Variables|Default|GetCamera%20Component))
  (bind _mouse_delta (Variables|MouseInput|GetMouse%20Delta))
  (bind (_x _y) (Math|Vector2D|BreakVector2D _mouse_delta))
  (Variables|Default|GetPhysics%20Handler
    (:then
      (Variables|Default|GetCamera%20Component
        (:then
          (Physics|Components|PhysicsHandle|SetTargetLocation (Variables|Default|GetPhysics%20Handler) (+ (Transformation|GetWorldLocation _camera_component) (* (Math|Vector|GetForwardVector _camera_component) (Variables|ObjectProperty|GetInteractOffsetValue))))
          (if (Variables|ObjectState|GetInInspection)
            (Class|PhysicsHandleComponent|SetTargetRotation (Variables|Default|GetPhysics%20Handler) (Math|Rotator|CombineRotators (.TargetRotation (Class|PhysicsHandleComponent|GetTargetLocationandRotation (Variables|Default|GetPhysics%20Handler))) (Math|Rotator|MakeRotator 0.0 _y _x)))))
        (:else)))
    (:else)))

(fn OnStoodon
  (bind _ownerstaticmesh (Variables|Default|GetOwnerStaticMesh))
  (bind _returnvalue (Transformation|GetWorldLocation _ownerstaticmesh))
  (bind (_outhit _returnvalue_2) (Collision|LineTraceByChannel _returnvalue (+ (* (Math|Vector|GetUpVector (Variables|/Script/Engine.Actor|GetRootComponent (Variables|Owner|GetOwnerActor))) (* (.z (Transformation|GetWorldScale (Variables|Default|GetOwnerStaticMesh))) (* -1.0 (Variables|ObjectProperty|GetActorBelowCheckLength)))) _returnvalue) "TraceTypeQuery1" false 0 "None"))
  (if _returnvalue_2
    (if (!= (.HitActor (Collision|BreakHitResult _outhit)) (Variables|SupportingActor|GetSupportingActor))
      (Physics|SetSimulatePhysics (Variables|Default|GetOwnerStaticMesh) false)
      (Utilities|IsValid (Actor|GetComponentbyClass (.HitActor (Collision|BreakHitResult _outhit)) "BPC_InteractableComponent_C")
        (:Is%20Valid
          (Class|BPIInteraction|Stoodon(Message) (Actor|GetComponentbyClass (.HitActor (Collision|BreakHitResult _outhit)) "BPC_InteractableComponent_C"))
          (Variables|SupportingActor|SetSupportingActor (.HitActor (Collision|BreakHitResult _outhit))))))
    (else
      (Physics|SetSimulatePhysics (Variables|Default|GetOwnerStaticMesh) true))))

(fn GetCanInteract
  (return (Variables|ObjectState|GetCanInteract)))