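; Base NPC student that performs daily routine actions: sleeping, following Mother Marry, queuing for food and sitting.
; BeginPlay sets the name widget, caches Mother Marry, chairs and food counter, and marks its bed occupied.
; Callable events use AIMoveTo, then interface messages to interact; seating retries random chairs until one is free.
; Helpers supply follow points on Mother Marry's spline, smoothly face her, and attach or destroy a food tray.
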(event Custom|BreakFast
  (Utilities|FlowControl|Sequence
    (:then_0
      ;[1 1 1] Go To BreakFast Hall
      (AI|AIMoveTo self (Variables|Default|GetCantin%20LOC) 0 5.0 false))
    (:then_1
      ;[1 1 1] Go To The Counter
      (AI|AIMoveTo self (Variables|Default|GetCantin%20Food%20Counter%20LOC) 0 5.0 false
        (:OnSuccess
          (Transformation|SetActorRotation "0, 0, 0"))))
    (:then_3
      ;[1 1 1] Go to The Sit
      (AI|AIMoveTo self (Variables|Default|GetTable%20LOC) 0 5.0 false))))

(event EventBeginPlay
  (Utilities|FlowControl|Sequence
    (:then_0
      (Class|BPIAI|SetAIDetails(Message) (UserInterface|GetWidget (Variables|Default|GetWidget)) (Variables|Default|GetStudentName) false))
    (:then_1
      (bind _returnvalue (Actor|GetActorOfClass "/Game/AI/Blueprints/BP_MotherMarry.BP_MotherMarry_C"))
      (Variables|Default|SetMotherMarryRef _returnvalue))
    (:then_2
      (bind _outactors (Actor|GetAllActorsOfClass "/Game/AI/Blueprints/Interactable/BP_Chair.BP_Chair_C"))
      (Variables|Default|SetChairRef _outactors))
    (:then_3
      (bind _returnvalue_2 (Actor|GetActorOfClass "/Game/AI/Blueprints/Interactable/BP_FoodCounter.BP_FoodCounter_C"))
      (Variables|Default|SetFood%20Counter%20Ref _returnvalue_2))
    (:then_4
      (bind _outactors_2 (Actor|GetAllActorsOfClass "/Game/AI/Blueprints/Interactable/BP_TableChair.BP_TableChair_C"))
      (Variables|Default|SetFoodTableRef _outactors_2))
    (:then_5
      (Variables|/Game/AI/Blueprints/Interactable/BP_InteractableOBJ.BP_InteractableOBJ_C|SetOccupied (Variables|Default|GetBed) true))
    (:then_6
      (Utilities|FlowControl|Delay 2.0))))

(event EventSitonChair
  (params (Duration :type Float%20%28double-precision%29) (IsFood%20Chair :type Boolean))
  ;[0 0 0] Sit On Chair
  (Variables|Default|SetDuration Duration)
  (Variables|Default|SetIs%20Food%20Chair IsFood%20Chair)
  (bind _output_get (Variables|Default|SetInteractableOBJ (Utilities|Array|Get(acopy) (select (Variables|Default|GetIs%20Food%20Chair) (Variables|Default|GetFoodTableRef) (Variables|Default|GetChairRef)) (Math|Random|RandomInteger (Utilities|Array|Length (select (Variables|Default|GetIs%20Food%20Chair) (Variables|Default|GetFoodTableRef) (Variables|Default|GetChairRef))))) :!label _label))
  (bind _yes_no (Class|BPIObjectInteraction|IsAvailable?(Message) _output_get))
  (if _yes_no
    (Class|BPIObjectInteraction|MarkasOccuiped(Message) _output_get)
    (AI|AIMoveTo self "0, 0, 0" _output_get 25.0 false
      (:OnSuccess
        (Class|BPIObjectInteraction|StartInteract(Message) (Variables|Default|GetInteractableOBJ) self)
        ;[0 0 0] End
        (if (Variables|Default|GetIs%20Food%20Chair)
          (Utilities|FlowControl|Delay (Variables|Default|GetDuration))
          (Class|BPIObjectInteraction|EndInteract(Message) (Variables|Default|GetInteractableOBJ)))))
    (else
      (Utilities|FlowControl|Delay 0.2)
      (goto _label))))

(event EventStandUp
  ;[0 0 0] End
  (Class|BPIObjectInteraction|EndInteract(Message) (Variables|Default|GetInteractableOBJ)))

(event EventGotoSleep
  ;[0 0 0] Sleep & Wake Up
  (AI|AIMoveTo self (Transformation|GetWorldLocation (Variables|/Game/AI/Blueprints/Interactable/BP_Bed.BP_Bed_C|GetStaticMesh (Variables|Default|GetBed))) 0 1.8e+02 false
    (:OnSuccess
      (Class|BPIObjectInteraction|StartInteract(Message) (Variables|Default|GetBed) self))))

(event EventFollowMother
  ;[0 0 0] Follow Mother Marry
  (AI|AIMoveTo self (CallFunction|GetLocationonSpline) 0 1e+01 false))

(event EventWakeUp
  ;[0 0 0] Sleep & Wake Up
  (Class|BPIObjectInteraction|EndInteract(Message) (Variables|Default|GetBed)))

(event EventGotoFoodCounter
  (params (Duration :type Float%20%28double-precision%29) (Delay%20Before%20Start :type Float%20%28double-precision%29) (LOC :type Vector :default "0, 0, 0"))
  ;[0 0 0] Food Counter
  (Utilities|FlowControl|Delay Delay%20Before%20Start)
  (AI|AIMoveTo self LOC 0 1.3e+02 false
    (:OnSuccess
      (Class|BPIObjectInteraction|StartInteract(Message) (Variables|Default|GetFood%20Counter%20Ref) self)
      (Utilities|FlowControl|Delay 0.2)
      (CallFunction|SitonChair Duration true))))

(event EventHoldPlate
  ;[0 0 0] Eating
  (bind _returnvalue (Game|SpawnActorfromClass "/Game/Assets/Models/FoodTray/BP_FoodTray.BP_FoodTray_C" (Math|Transform|MakeTransform "0, 0, 0" "0, 0, 0" "0.100000,0.100000,0.100000") "AlwaysSpawn" "MultiplyWithRoot" 0 0))
  (bind _output_get (Variables|Default|SetPlate%20Ref _returnvalue))
  (Transformation|AttachComponentToComponent _output_get (Variables|Character|GetMesh) "Plate" "SnapToTarget" "SnapToTarget" "SnapToTarget" true)
  (Variables|Default|SetHasPlate true))

(event EventDestroyPlate
  ;[0 0 0] Eating
  (Actor|DestroyActor (Variables|Default|GetPlate%20Ref)))

(fn ConstructionScript)

(fn GetLocationonSpline
  (return (Spline|GetLocationatSplinePoint (Variables|/Game/AI/Blueprints/BP_MotherMarry.BP_MotherMarry_C|GetS1 (Variables|Default|GetMotherMarryRef)) (Variables|Default|GetPoint) "World")))

(fn LookMotherMarry
  (Transformation|SetActorRotation (Math|Interpolation|RInterpTo (Transformation|GetActorRotation) (Math|Rotator|FindLookatRotation (Transformation|GetActorLocation) (Transformation|GetActorLocation (Variables|Default|GetMotherMarryRef))) (Utilities|Time|GetWorldDeltaSeconds) 8.0)))