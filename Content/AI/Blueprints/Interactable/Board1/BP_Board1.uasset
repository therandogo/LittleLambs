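; BP_Board1 is a paintable board that the player draws on by looking at it and using IA_Paint.
; BeginPlay creates a render target, feeds it into the mesh's M_canvas material and prepares an M_Brush instance.
; Painting traces from the camera, converts the hit to a UV, and DrawBrush stamps the colored brush there via render-target canvas drawing.
; An older M_Marker and RT_Board drawing path is left disconnected.
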(event Input|EnhancedActionEvents|EnhancedInputActionIA_Paint
  (params (ActionValue :type Float%20%28double-precision%29) (ElapsedSeconds :type Float%20%28double-precision%29) (TriggeredSeconds :type Float%20%28double-precision%29) (InputAction :type Input%20Action%20Object%20Reference :default "/Game/ThirdPerson/Input/IA_Paint.IA_Paint"))
  (bind _returnvalue (Game|GetPlayerCameraManager 0))
  (bind _returnvalue_2 (Transformation|GetActorLocation _returnvalue))
  (if (== ActionValue 1.0)
    (bind _outhit (Collision|LineTraceByChannel _returnvalue_2 (+ _returnvalue_2 (* (Transformation|GetActorForwardVector _returnvalue) 5e+02)) "TraceTypeQuery1" true (Utilities|Array|MakeArray (Game|GetPlayerCharacter 0)) "None" false))
    (if (== (.HitActor (Collision|BreakHitResult _outhit)) self)
      (CallFunction|DrawBrush (Variables|Default|GetPaint%20Brush%20Size) (.UV (Class|GameplayStatics|FindCollisionUV _outhit)) (Variables|Default|GetPaint%20Color)))))

(event EventBeginPlay
  (Utilities|FlowControl|Sequence
    (:then_0
      (Utilities|FlowControl|Sequence
        (:then_0
          (bind _returnvalue (Rendering|CreateRenderTarget2D 1024 1024 "RTF_RGBA16f"))
          (bind _output_get (Variables|Default|SetRender%20Target _returnvalue))
          (Rendering|ClearRenderTarget2D _output_get "(R=0.000000,G=0.000000,B=0.000000,A=0.000000)"))
        (:then_1
          (bind _returnvalue_2 (Rendering|Material|CreateDynamicMaterialInstance "/Game/AI/Blueprints/Interactable/Board1/M_canvas.M_canvas" "None" "None" :!class /Script/Engine.KismetMaterialLibrary))
          (Rendering|Material|SetTextureParameterValue _returnvalue_2 "RanderTarget" (Variables|Default|GetRender%20Target))
          (Rendering|Material|SetMaterial (Variables|Default|GetStaticMesh) 0 _returnvalue_2))
        (:then_2
          (bind _returnvalue_3 (Rendering|Material|CreateDynamicMaterialInstance "/Game/AI/Blueprints/Interactable/Board1/M_Brush.M_Brush" "None" "None" :!class /Script/Engine.KismetMaterialLibrary))
          (Variables|Default|SetBrushMaterial _returnvalue_3))))))

(fn ConstructionScript
  (|CallParentFunction))

(fn DrawBrush
  (params (Brush%20Size :type Float%20%28double-precision%29) (Draw%20Location :type Vector%202D%20Structure) (Color :type Linear%20Color%20Structure))
  (bind _paint_brush_size (Variables|Default|GetPaint%20Brush%20Size))
  (Utilities|FlowControl|Sequence
    (:then_0
      (Rendering|Material|SetVectorParameterValue (Variables|Default|GetBrushMaterial) "Brush Color" Color :!class /Script/Engine.MaterialInstanceDynamic))
    (:then_1
      (bind (_canvas _size _context) (Rendering|BeginDrawCanvastoRenderTarget (Variables|Default|GetRender%20Target)))
      (Canvas|DrawMaterial :self _canvas :RenderMaterial (Variables|Default|GetBrushMaterial) :ScreenPosition (+ (- (* _size Draw%20Location) (/ Brush%20Size 2.0)) "(X=0.000000,Y=12.500000)") :ScreenSize (Math|Vector2D|MakeVector2D _paint_brush_size (/ _paint_brush_size 2.0)) :CoordinateSize "(X=1.000000,Y=1.000000)" :PivotPoint "(X=0.500000,Y=0.500000)")
      (Rendering|EndDrawCanvastoRenderTarget _context))))