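; BP_Bed is an interactable bed that a character can lie down and sleep on.
; Two start events (one fetches the player character, the other takes the interacting actor) share logic that disables movement, plays the Sleep montage and eases the capsule onto the bed.
; Both stop events play a StandUP montage, then on completion move the character to the StandLOC point and re-enable movement.
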(event EventBeginPlay
  (|CallParentFunction) ; This node is disabled and will not be called.\nDrag off pins to build functionality.
)

(event Collision|EventActorBeginOverlap
  (params (OtherActor :type Actor%20Object%20Reference))
  (|CallParentFunction OtherActor) ; This node is disabled and will not be called.\nDrag off pins to build functionality.
)

(event EventTick
  (params (DeltaSeconds :type Float%20%28single-precision%29))
  (|CallParentFunction DeltaSeconds) ; This node is disabled and will not be called.\nDrag off pins to build functionality.
)

(event EventStartInteracting
  (|CallParentFunction)
  (bind _character (Class|BPIPlayer|PlayerData(Message) (Variables|Default|GetActor%20Ref)))
  (bind _output_get (Variables|Default|SetCharacter _character))
  (Class|BPIPlayer|ToggleMovement(Message) _output_get false)
  (Animation|PlayAnimMontage (Variables|Default|GetCharacter) "/Game/Assets/Animations/Sleep.Sleep" 1.0 "None")
  (Components|MoveComponentTo (Variables|/Script/Engine.Actor|GetRootComponent (Variables|Default|GetCharacter)) (+ (Transformation|GetActorLocation) (Math|Vector|MakeVector 0.0 0.0 (+ (Variables|/Script/Engine.CapsuleComponent|GetCapsuleHalfHeight (Variables|/Script/Engine.Character|GetCapsuleComponent (Variables|Default|GetCharacter))) -15.0))) (Math|Rotator|MakeRotator 0.0 0.0 (.yaw (Transformation|GetActorRotation))) true true 0.5 true))

(event EventStartInteract
  (params (Interacting%20Actor :type Character%20Object%20Reference))
  (|CallParentFunction Interacting%20Actor)
  (bind _output_get (Variables|Default|SetCharacter (Variables|Default|GetInteracting%20Actor)))
  (Class|BPIPlayer|ToggleMovement(Message) _output_get false)
  (Animation|PlayAnimMontage (Variables|Default|GetCharacter) "/Game/Assets/Animations/Sleep.Sleep" 1.0 "None")
  (Components|MoveComponentTo (Variables|/Script/Engine.Actor|GetRootComponent (Variables|Default|GetCharacter)) (+ (Transformation|GetActorLocation) (Math|Vector|MakeVector 0.0 0.0 (+ (Variables|/Script/Engine.CapsuleComponent|GetCapsuleHalfHeight (Variables|/Script/Engine.Character|GetCapsuleComponent (Variables|Default|GetCharacter))) -15.0))) (Math|Rotator|MakeRotator 0.0 0.0 (.yaw (Transformation|GetActorRotation))) true true 0.5 true))

(event EventEndInteract
  (bind _character (Variables|Default|GetCharacter))
  (|CallParentFunction)
  (bind _character_2 (Variables|Default|GetCharacter)
    (:then
      (Animation|Montage|PlayMontage (Variables|/Script/Engine.Character|GetMesh _character_2) "/Game/Assets/Animations/StandUP.StandUP"
        (:OnCompleted
          (Components|MoveComponentTo (Variables|/Script/Engine.Actor|GetRootComponent _character) (+ (Math|Vector|MakeVector 0.0 0.0 (Variables|/Script/Engine.CapsuleComponent|GetCapsuleHalfHeight (Variables|/Script/Engine.Character|GetCapsuleComponent _character))) (Transformation|GetWorldLocation (Variables|Default|GetStand%20LOC))) (Transformation|GetActorRotation _character) false false 0.5 false)
          (Class|BPIPlayer|ToggleMovement(Message) (Variables|Default|GetCharacter) true))))
    (:else)))

(event EventStopInteracting
  (bind _character (Variables|Default|GetCharacter))
  (|CallParentFunction)
  (bind _character_2 (Variables|Default|GetCharacter)
    (:then
      (Animation|Montage|PlayMontage (Variables|/Script/Engine.Character|GetMesh _character_2) "/Game/Assets/Animations/StandUP.StandUP"
        (:OnCompleted
          (Components|MoveComponentTo (Variables|/Script/Engine.Actor|GetRootComponent _character) (+ (Math|Vector|MakeVector 0.0 0.0 (Variables|/Script/Engine.CapsuleComponent|GetCapsuleHalfHeight (Variables|/Script/Engine.Character|GetCapsuleComponent _character))) (Transformation|GetWorldLocation (Variables|Default|GetStand%20LOC))) (Transformation|GetActorRotation _character) false false 0.5 false)
          (Class|BPIPlayer|ToggleMovement(Message) (Variables|Default|GetCharacter) true))))
    (:else)))

(fn ConstructionScript
  (|CallParentFunction))