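; BP_Toilet is an interactable toilet that flushes when interacted with, guarded by a CanFlush flag against repeat triggers.
; StartInteracting snaps the handle to a pitched angle, plays the toilet sound at the actor's location and starts a timer to the Restting event.
; Restting runs a timeline that lerps the handle back to rest, then re-enables flushing and adds a referenced widget to the viewport.
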(event Custom|Restting
  (bind _alpha (Timeline|Timeline PlayFromStart)
    (:Update
      (Transformation|SetRelativeRotation (Variables|Default|GetHandle) (Math|Rotator|MakeRotator 0.0 (Math|Float|Lerp 2e+01 0.0 _alpha) 0.0) false false))
    (:Finished
      (Variables|Default|SetCan%20Flush true)
      (UserInterface|Viewport|AddtoViewport (Variables|Default|GetWidgetRef) 0))))

(event EventBeginPlay
  (|CallParentFunction) ; This node is disabled and will not be called.\nDrag off pins to build functionality.
)

(event Collision|EventActorBeginOverlap
  (params (OtherActor :type Actor%20Object%20Reference)))

(event EventTick
  (params (DeltaSeconds :type Float%20%28single-precision%29)))

(event EventStartInteracting
  (if (Variables|Default|GetCan%20Flush)
    (Variables|Default|SetCan%20Flush false)
    (Transformation|SetRelativeRotation (Variables|Default|GetHandle) (Math|Rotator|MakeRotator 0.0 2e+01 0.0) false false)
    (Utilities|Time|SetTimerbyFunctionName 0 "Restting" 1.0)
    (Audio|PlaySoundatLocation "/Game/AI/Blueprints/Interactable/Toilet/Sound/Toilet.Toilet" (Transformation|GetActorLocation) "0, 0, 0" 1.0 1.0 0.0 0 0 0 0)))

(fn ConstructionScript
  (|CallParentFunction))