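; BP_SpinChair is an interactable chair that spins around its yaw axis when used.
; Each StartInteracting call adds SpinMultiplier to SpinSpeed, clamped to a fixed range.
; Tick rotates the whole actor by SpinSpeed scaled by delta time.
; A latent Delay inside Tick throttles the Friction multiplier to roughly fixed intervals, so the spin changes in steps independently of the per-frame rotation.
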(event EventBeginPlay
  (|CallParentFunction) ; This node is disabled and will not be called.\nDrag off pins to build functionality.
)

(event Collision|EventActorBeginOverlap
  (params (OtherActor :type Actor%20Object%20Reference)))

(event EventTick
  (params (DeltaSeconds :type Float%20%28single-precision%29))
  (Transformation|AddActorLocalRotation (Math|Rotator|MakeRotator 0.0 0.0 (* DeltaSeconds (Variables|Default|GetSpinSpeed))) false false)
  (Utilities|FlowControl|Delay 0.2)
  (Variables|Default|SetSpinSpeed (* (Variables|Default|GetSpinSpeed) (Variables|Default|GetFriction))))

(event EventStartInteracting
  (Variables|Default|SetSpinSpeed (Math|Float|Clamp(Float) (+ (Variables|Default|GetSpinSpeed) (Variables|Default|GetSpinMultiplier)) 0.0 1e+03)))

(fn ConstructionScript
  (|CallParentFunction))