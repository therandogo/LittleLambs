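; BP_InteractableOBJ is an interactable world object, such as a food table, chair, bed, class table or food counter, that tracks whether it is occupied.
; Player overlap with its box shows an instruction widget and enables input when the EIType rule passes; class tables never qualify, and food counters also check HasPlateMessage.
; E toggles interaction, while StartInteract, EndInteract, MarkasOccuiped and IsAvailable let other actors share the same occupancy state.
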(event OnComponentBeginOverlap(Box)
  (params (OverlappedComponent :type Primitive%20Component%20Object%20Reference) (OtherActor :type Actor%20Object%20Reference) (OtherComp :type Primitive%20Component%20Object%20Reference) (OtherBodyIndex :type Integer) (bFromSweep :type Boolean) (SweepResult :type Hit%20Result%20Structure%20%28by%20ref%29))
  (bind _occupied (Variables|Default|GetOccupied))
  (bind _returnvalue (not _occupied))
  (bind _has_plate (Class|BPIPlayer|HasPlate(Message) OtherActor))
  (if (Utilities|Select :Index (Variables|Default|GetE_IType) :NewEnumerator0 _returnvalue :NewEnumerator1 _returnvalue :NewEnumerator2 _returnvalue :NewEnumerator3 false :NewEnumerator4 (and _returnvalue (not _has_plate)))
    (if (== OtherActor (Game|GetPlayerCharacter 0))
      (Variables|Default|SetActor%20Ref OtherActor)
      (UserInterface|Viewport|AddtoViewport (Variables|Default|GetWidgetRef) 0)
      (Input|EnableInput (Game|GetPlayerController 0)))))

(event OnComponentEndOverlap(Box)
  (params (OverlappedComponent :type Primitive%20Component%20Object%20Reference) (OtherActor :type Actor%20Object%20Reference) (OtherComp :type Primitive%20Component%20Object%20Reference) (OtherBodyIndex :type Integer))
  (if (== OtherActor (Game|GetPlayerCharacter 0))
    (Widget|RemovefromParent (Variables|Default|GetWidgetRef))
    (Input|DisableInput (Game|GetPlayerController 0))))

(event Custom|Stop%20Interacting
  (Variables|Default|SetInteracting false)
  (Variables|Default|SetOccupied false))

(event Custom|Start%20Interacting
  (Variables|Default|SetOccupied true)
  (Variables|Default|SetInteracting true))

(event EventBeginPlay
  (bind _returnvalue (UserInterface|CreateWidget "/Game/AI/Widgets/WBP_Instruction.WBP_Instruction_C"))
  (Variables|Default|SetWidgetRef _returnvalue))

(event EventEndInteract
  (Variables|Default|SetInteracting false)
  (Variables|Default|SetOccupied false))

(event EventStartInteract
  (params (Interacting%20Actor :type Character%20Object%20Reference))
  (Variables|Default|SetInteracting%20Actor Interacting%20Actor)
  (Variables|Default|SetOccupied true)
  (Variables|Default|SetInteracting true))

(event EventMarkasOccuiped
  (Variables|Default|SetOccupied true))

(event Input|KeyboardEvents|E
  (params (Key :type Key%20Structure :default "None"))
  (:Pressed
    (if (Variables|Default|GetInteracting)
      (CallFunction|StopInteracting)
      (else
        (CallFunction|StartInteracting)
        (Widget|RemovefromParent (Variables|Default|GetWidgetRef))))))

(fn ConstructionScript)

(fn IsAvailable?
  (return (not (Variables|Default|GetOccupied))))