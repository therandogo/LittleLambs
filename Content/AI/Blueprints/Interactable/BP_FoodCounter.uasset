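; BP_FoodCounter is an interactable food counter that has the interacting character hold a plate.
; StartInteracting gets the character through a PlayerData message, while StartInteract takes the passed-in actor, and both share one path.
; That path starts a walking montage on the character's mesh and immediately sends HoldPlate, with a player-character check whose two branches make the same call.
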(event EventBeginPlay
  (|CallParentFunction) ; This node is disabled and will not be called.\nDrag off pins to build functionality.
)

(event Collision|EventActorBeginOverlap
  (params (OtherActor :type Actor%20Object%20Reference))
  (|CallParentFunction OtherActor) ; This node is disabled and will not be called.\nDrag off pins to build functionality.
)

(event EventTick
  (params (DeltaSeconds :type Float%20%28single-precision%29))
  (|CallParentFunction DeltaSeconds) ; This node is disabled and will not be called.\nDrag off pins to build functionality.
)

(event EventStartInteracting
  (bind _character (Class|BPIPlayer|PlayerData(Message) (Variables|Default|GetActor%20Ref)))
  (Variables|Default|SetCharacter _character)
  (Animation|Montage|PlayMontage (Variables|/Script/Engine.Character|GetMesh (Variables|Default|GetCharacter)) "/Game/Assets/Animations/Walking_UE5_Montage.Walking_UE5_Montage"
    (:then
      (if (== (Variables|Default|GetCharacter) (Game|GetPlayerCharacter 0))
        (Class|BPIPlayer|HoldPlate(Message) (Variables|Default|GetCharacter))
        (else
          (Class|BPIAI|HoldPlate(Message) (Variables|Default|GetCharacter)))))))

(event EventStartInteract
  (params (Interacting%20Actor :type Character%20Object%20Reference))
  (Variables|Default|SetCharacter Interacting%20Actor)
  (Animation|Montage|PlayMontage (Variables|/Script/Engine.Character|GetMesh (Variables|Default|GetCharacter)) "/Game/Assets/Animations/Walking_UE5_Montage.Walking_UE5_Montage"
    (:then
      (if (== (Variables|Default|GetCharacter) (Game|GetPlayerCharacter 0))
        (Class|BPIPlayer|HoldPlate(Message) (Variables|Default|GetCharacter))
        (else
          (Class|BPIAI|HoldPlate(Message) (Variables|Default|GetCharacter)))))))

(fn ConstructionScript
  (|CallParentFunction))