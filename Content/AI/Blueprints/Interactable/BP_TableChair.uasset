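; Interactable table chair that seats the player or another character, placing a food tray on the table.
; Both start-interact events lock movement, play a sitting montage and ease the character onto the seat.
; Players get a tray at TrayLOC only when carrying a plate, which is destroyed; other characters always get one.
; Both end events stop the montage, move the character to StandLOC and restore movement.
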(event EventBeginPlay
  (|CallParentFunction) ; This node is disabled and will not be called.\nDrag off pins to build functionality.
)

(event Collision|EventActorBeginOverlap
  (params (OtherActor :type Actor%20Object%20Reference))
  (|CallParentFunction OtherActor) ; This node is disabled and will not be called.\nDrag off pins to build functionality.
)

(event EventTick
  (params (DeltaSeconds :type Float%20%28single-precision%29))
  (|CallParentFunction DeltaSeconds) ; This node is disabled and will not be called.\nDrag off pins to build functionality.
)

(event EventStartInteracting
  (|CallParentFunction)
  (bind _character (Class|BPIPlayer|PlayerData(Message) (Variables|Default|GetActor%20Ref)))
  (bind _output_get (Variables|Default|SetCharacter _character))
  (Class|BPIPlayer|ToggleMovement(Message) _output_get false)
  (if (== (Game|GetPlayerCharacter 0) (Variables|Default|GetCharacter))
    (bind _has_plate (Class|BPIPlayer|HasPlate(Message) (Variables|Default|GetCharacter)))
    (if _has_plate
      (Class|BPIPlayer|DestroyPlate(Message) (Variables|Default|GetCharacter))
      (Game|SpawnActorfromClass "/Game/Assets/Models/FoodTray/BP_FoodTray.BP_FoodTray_C" (Math|Transform|MakeTransform (Transformation|GetWorldLocation (Variables|Default|GetTray%20LOC)) "0, 0, 0" "0.500000,0.500000,0.500000") "Undefined" "MultiplyWithRoot" 0 0 :!label _label))
    (else
      (Class|BPIAI|DestroyPlate(Message) (Variables|Default|GetCharacter))
      (goto _label)))
  (Animation|PlayAnimMontage (Variables|Default|GetCharacter) "/Game/Assets/Animations/Sitting.Sitting" 1.0 "None")
  (Components|MoveComponentTo (Variables|/Script/Engine.Actor|GetRootComponent (Variables|Default|GetCharacter)) (+ (Transformation|GetActorLocation) (Math|Vector|MakeVector 0.0 0.0 (Variables|/Script/Engine.CapsuleComponent|GetCapsuleHalfHeight (Variables|/Script/Engine.Character|GetCapsuleComponent (Variables|Default|GetCharacter))))) (Math|Rotator|MakeRotator 0.0 0.0 (.yaw (Transformation|GetActorRotation))) true true 0.5 true))

(event EventStopInteracting
  (bind _character (Variables|Default|GetCharacter))
  (|CallParentFunction)
  (bind _character_2 (Variables|Default|GetCharacter)
    (:then
      (Animation|StopAnimMontage _character_2 "/Game/Assets/Animations/Sitting.Sitting")
      (Components|MoveComponentTo (Variables|/Script/Engine.Actor|GetRootComponent _character) (+ (Math|Vector|MakeVector 0.0 0.0 (Variables|/Script/Engine.CapsuleComponent|GetCapsuleHalfHeight (Variables|/Script/Engine.Character|GetCapsuleComponent _character))) (Transformation|GetWorldLocation (Variables|Default|GetStand%20LOC))) (Transformation|GetActorRotation _character) false false 0.5 false)
      (Class|BPIPlayer|ToggleMovement(Message) (Variables|Default|GetCharacter) true))
    (:else)))

(event EventEndInteract
  (bind _character (Variables|Default|GetCharacter))
  (|CallParentFunction)
  (bind _character_2 (Variables|Default|GetCharacter)
    (:then
      (Animation|StopAnimMontage _character_2 "/Game/Assets/Animations/Sitting.Sitting")
      (Components|MoveComponentTo (Variables|/Script/Engine.Actor|GetRootComponent _character) (+ (Math|Vector|MakeVector 0.0 0.0 (Variables|/Script/Engine.CapsuleComponent|GetCapsuleHalfHeight (Variables|/Script/Engine.Character|GetCapsuleComponent _character))) (Transformation|GetWorldLocation (Variables|Default|GetStand%20LOC))) (Transformation|GetActorRotation _character) false false 0.5 false)
      (Class|BPIPlayer|ToggleMovement(Message) (Variables|Default|GetCharacter) true))
    (:else)))

(event EventStartInteract
  (params (Interacting%20Actor :type Character%20Object%20Reference))
  (|CallParentFunction Interacting%20Actor)
  (bind _output_get (Variables|Default|SetCharacter (Variables|Default|GetInteracting%20Actor)))
  (Class|BPIPlayer|ToggleMovement(Message) _output_get false)
  (if (== (Game|GetPlayerCharacter 0) (Variables|Default|GetCharacter))
    (bind _has_plate (Class|BPIPlayer|HasPlate(Message) (Variables|Default|GetCharacter)))
    (if _has_plate
      (Class|BPIPlayer|DestroyPlate(Message) (Variables|Default|GetCharacter))
      (Game|SpawnActorfromClass "/Game/Assets/Models/FoodTray/BP_FoodTray.BP_FoodTray_C" (Math|Transform|MakeTransform (Transformation|GetWorldLocation (Variables|Default|GetTray%20LOC)) "0, 0, 0" "0.500000,0.500000,0.500000") "Undefined" "MultiplyWithRoot" 0 0 :!label _label))
    (else
      (Class|BPIAI|DestroyPlate(Message) (Variables|Default|GetCharacter))
      (goto _label)))
  (Animation|PlayAnimMontage (Variables|Default|GetCharacter) "/Game/Assets/Animations/Sitting.Sitting" 1.0 "None")
  (Components|MoveComponentTo (Variables|/Script/Engine.Actor|GetRootComponent (Variables|Default|GetCharacter)) (+ (Transformation|GetActorLocation) (Math|Vector|MakeVector 0.0 0.0 (Variables|/Script/Engine.CapsuleComponent|GetCapsuleHalfHeight (Variables|/Script/Engine.Character|GetCapsuleComponent (Variables|Default|GetCharacter))))) (Math|Rotator|MakeRotator 0.0 0.0 (.yaw (Transformation|GetActorRotation))) true true 0.5 true))

(fn ConstructionScript
  (|CallParentFunction))