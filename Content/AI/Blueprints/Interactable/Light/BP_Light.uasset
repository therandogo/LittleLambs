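; BP_Light is an interactable point light that switches on or off through an On/OffLight event, ignored when Dead.
; The construction script sets its colour and attenuation radius and starts it at zero intensity.
; With Flicker set, switching on applies a flicker light-function material and spawns a sound, and switching off zeroes intensity and stops the sound.
; Otherwise, each switch sets intensity and applies the flicker material briefly before clearing it.
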(event Custom|On/Off%20Light
  (params (On :type Boolean))
  (if (not (Variables|Default|GetDead))
    (if (Variables|Default|GetFlicker)
      (if On
        (Rendering|Components|Light|SetLightFunctionMaterial (Variables|Default|GetPointLight) "/Game/AI/Blueprints/Interactable/Light/Material/M_Flicker.M_Flicker")
        (bind _returnvalue (Audio|SpawnSoundatLocation "/Game/AI/Blueprints/Interactable/Light/Sounds/Flicker.Flicker" (Transformation|GetActorLocation) "0, 0, 0" 1.0 1.0 0.0 0 0))
        (Rendering|Components|Light|SetIntensity (Variables|Default|GetPointLight) (Variables|Default|GetIntensity))
        (else
          (Rendering|Components|Light|SetIntensity (Variables|Default|GetPointLight) 0.0)
          (Audio|Components|Audio|Stop _returnvalue)))
      (else
        (Rendering|Components|Light|SetIntensity (Variables|Default|GetPointLight) (select On (Variables|Default|GetIntensity) 0.0))
        (Rendering|Components|Light|SetLightFunctionMaterial (Variables|Default|GetPointLight) "/Game/AI/Blueprints/Interactable/Light/Material/M_Flicker.M_Flicker")
        (Utilities|FlowControl|Delay 0.5)
        (Rendering|Components|Light|SetLightFunctionMaterial (Variables|Default|GetPointLight) 0)))))

(fn ConstructionScript
  (bind _pointlight (Variables|Default|GetPointLight))
  (Rendering|Components|Light|SetLightColor _pointlight (Variables|Default|GetLight%20Color) true)
  (Rendering|Components|Light|SetIntensity _pointlight 0.0)
  (Rendering|Lighting|SetAttenuationRadius _pointlight (Variables|Default|GetAttenuation%20Radius)))