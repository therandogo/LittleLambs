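; BP_LightSwitch is an interactable wall-switch style Blueprint that turns its referenced Light on and off.
; Each StartInteracting event runs a FlipFlop that alternately calls OnOffLight with true or false on that Light.
; The same toggle state tilts the Switch component's pitch one way or the other, then a click sound plays at the actor's location.
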(event EventBeginPlay
  (|CallParentFunction) ; This node is disabled and will not be called.\nDrag off pins to build functionality.
)

(event Collision|EventActorBeginOverlap
  (params (OtherActor :type Actor%20Object%20Reference)))

(event EventTick
  (params (DeltaSeconds :type Float%20%28single-precision%29)))

(event EventStartInteracting
  (bind _light (Variables|Default|GetLight))
  (bind _isa (Utilities|FlowControl|FlipFlop)
    (:A
      (Default|On/OffLight _light true))
    (:B
      (Default|On/OffLight _light false)))
  (Transformation|SetRelativeRotation (Variables|Default|GetSwitch) (Math|Rotator|MakeRotator 0.0 (select _isa -8.0 8.0) 0.0) false false)
  (Audio|PlaySoundatLocation "/Game/AI/Blueprints/Interactable/Light/Sounds/LightSwitch.LightSwitch" (Transformation|GetActorLocation) "0, 0, 0" 1.5 1.0 0.0 0 0 0 0))

(fn ConstructionScript
  (|CallParentFunction))