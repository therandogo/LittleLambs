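; BP_MotherMarry is a teacher NPC that waits for two lanes of NPCs and the player to line up before walking forward.
; Tick checks NPCs against their spline points until IsInLine latches; each element overwrites the flag, so the last one checked decides.
; Once that is set and the player nears S2's first point, she AI-moves along her forward vector.
; Otherwise movement is disabled and a spawned Location marker shows that point.
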(event EventBeginPlay
  (Class|BPIAI|SetAIDetails(Message) (UserInterface|GetWidget (Variables|Default|GetWidget)) "Mother Marry" true)
  (bind _returnvalue (Game|SpawnActorfromClass "/Game/AI/Blueprints/Location.Location_C" (Math|Transform|MakeTransform "0, 0, 0" "0, 0, 0" "1.000000,1.000000,1.000000") "Undefined" "MultiplyWithRoot" 0 0))
  (Variables|Default|SetRef _returnvalue))

(event EventTick
  (params (DeltaSeconds :type Float%20%28single-precision%29))
  (bind _s2 (Variables|Default|GetS2))
  (bind _returnvalue (Spline|GetLocationatSplinePoint _s2 0 "World"))
  (Utilities|FlowControl|Sequence
    (:then_0
      (if (not (Variables|Default|GetIs%20In%20Line))
        (CallFunction|Check (Variables|Default|GetLane%201%20NPC))
        (CallFunction|Check (Variables|Default|GetLane%202%20NPC))))
    (:then_1
      (if (and (< (Math|Vector|Distance(Vector) (Transformation|GetActorLocation (Game|GetPlayerCharacter 0)) (Spline|GetLocationatSplinePoint (Variables|Default|GetS2) 0 "World")) 2e+02) (Variables|Default|GetIs%20In%20Line))
        (Pawn|Components|CharacterMovement|SetMovementMode (Variables|Character|GetCharacterMovement) "MOVE_Walking" 0)
        (Rendering|SetActorHiddenInGame (Variables|Default|GetRef) true)
        (AI|AIMoveTo self (+ (Transformation|GetActorLocation) (* (Transformation|GetActorForwardVector) 4e+03)) 0 5.0 false)
        (else
          (Pawn|Components|CharacterMovement|SetMovementMode (Variables|Character|GetCharacterMovement) "MOVE_None" 0)
          (Rendering|SetActorHiddenInGame (Variables|Default|GetRef) false)
          (Transformation|SetActorLocation (Variables|Default|GetRef) (Math|Vector|MakeVector (.x _returnvalue) (.y _returnvalue) 5.0) false false))))))

(fn ConstructionScript)

(fn Check
  (params (Array :type Array%20of%20BP%20NPC%20Base%20Object%20References))
  (for _array_element Array
    (if (<= (Math|Vector|Distance(Vector) (Transformation|GetActorLocation _array_element) (Spline|GetLocationatSplinePoint (select (Variables|/Game/AI/Blueprints/BP_NPC_Base.BP_NPC_Base_C|GetLane1 _array_element) (Variables|Default|GetS1) (Variables|Default|GetS2)) (Variables|/Game/AI/Blueprints/BP_NPC_Base.BP_NPC_Base_C|GetPoint _array_element) "World")) 55.0)
      (Variables|Default|SetIs%20In%20Line true)
      (else
        (Variables|Default|SetIs%20In%20Line false)))))