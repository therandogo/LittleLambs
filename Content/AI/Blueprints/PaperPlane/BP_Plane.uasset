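; Paper plane actor that launches along X with ProjectileMovement, then wobbles and gradually loses speed and height.
; A timeline blends in random Y/Z local drift, using a flag to pick new offsets.
; Its updates start a second timeline that jitters pitch and yaw with values re-rolled each update.
; That chains through a five-second delay into a third timeline that lowers forward velocity and raises gravity scale.
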(event EventBeginPlay
  (Variables|/Script/Engine.MovementComponent|SetVelocity (Variables|Default|GetProjectileMovement) "1000.000000,0.000000,0.000000")
  (bind _newtrack_0 (Timeline|Timeline Play)
    (:Update
      (if (Variables|Default|Getb)
        (Variables|Default|Setb false)
        (Variables|Default|SetNewVar (Math|Random|RandomFloatinRange -1.0 1.0))
        (Variables|Default|SetNewVar_0 (Math|Random|RandomFloatinRange -1.0 1.0)))
      (Transformation|AddActorLocalOffset (Math|Vector|MakeVector 0.0 (Math|Float|Lerp 0.0 (Variables|Default|GetNewVar) _newtrack_0) (Math|Float|Lerp 0.0 (Variables|Default|GetNewVar_0) _newtrack_0)) false false)
      (bind _newtrack_0_2 (Timeline|Timeline_1 Play)
        (:Update
          (Transformation|SetActorRotation (Math|Rotator|MakeRotator 0.0 (Math|Float|Lerp 0.0 (Math|Random|RandomFloatinRange -1.0 1.0) _newtrack_0_2) (Math|Float|Lerp 0.0 (Math|Random|RandomFloatinRange -2.0 2.0) _newtrack_0_2)))
          (Utilities|FlowControl|Delay 5.0)
          (bind _newtrack_0_3 (Timeline|Timeline_0 Play)
            (:Update
              (Variables|/Script/Engine.MovementComponent|SetVelocity (Variables|Default|GetProjectileMovement) (Math|Vector|MakeVector (Math|Float|Lerp 2.5e+02 1.5e+02 _newtrack_0_3) 0.0 (Math|Float|Lerp 0.0 -1.0 _newtrack_0_3)))
              (Variables|/Script/Engine.ProjectileMovementComponent|SetProjectileGravityScale (Variables|Default|GetProjectileMovement) (Math|Float|Lerp 0.01 0.05 _newtrack_0_3)))))))
    (:Finished
      (Variables|Default|Setb true))))

(fn ConstructionScript)