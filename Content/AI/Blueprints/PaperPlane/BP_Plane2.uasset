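; BP_Plane2 is a paper plane actor that flies in the direction of the player controller's aim.
; It starts with zero velocity; StartTimer detaches the given component and starts a fast looping timer, guarded against duplicates.
; Each tick of that timer copies control pitch and yaw to the plane and sets constant forward velocity, until ClearTimer stops it.
; Interacting calls SpawnPlaneMessage on the player character and destroys the plane.
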(event Custom|ClearTimer
  (Utilities|Time|ClearandInvalidateTimerbyHandle (Variables|Default|GetTimerRef)))

(event Custom|Start%20Timer
  (params (Attach :type Arrow%20Component%20Object%20Reference))
  (if (not (Utilities|Time|IsValidTimerHandle (Variables|Default|GetTimerRef)))
    (Transformation|DetachFromComponent Attach "KeepWorld" "KeepWorld" "KeepWorld" true)
    (bind _returnvalue (Utilities|Time|SetTimerbyFunctionName 0 "UpdateDirection" 0.01 true))
    (Variables|Default|SetTimerRef _returnvalue)))

(event EventBeginPlay
  (|CallParentFunction)
  (Variables|/Script/Engine.MovementComponent|SetVelocity (Variables|Default|GetProjectileMovement1) "0, 0, 0")
  (Variables|Default|SetIsSpawned (Variables|Default|GetPlane%20Is%20Spawned)))

(event EventStartInteracting
  (Class|BPIPlayer|SpawnPlane(Message) (Game|GetPlayerCharacter 0))
  (Actor|DestroyActor))

(fn ConstructionScript)

(fn UpdateDirection
  (bind _returnvalue (Game|GetPlayerController 0))
  (bind _returnvalue_2 (Transformation|GetActorRotation))
  (bind _returnvalue_3 (Pawn|GetControlRotation _returnvalue :!class /Script/Engine.Controller))
  (bind _returnvalue_4 (Math|Vector|GetForwardVector _returnvalue_2))
  (Transformation|SetActorRotation (Math|Rotator|MakeRotator 0.0 (.pitch _returnvalue_3) (.yaw _returnvalue_3)))
  (Variables|/Script/Engine.MovementComponent|SetVelocity (Variables|Default|GetProjectileMovement1) (Math|Vector|MakeVector (* (.x _returnvalue_4) 1e+02) (* (.y _returnvalue_4) 1e+02) (* (.z _returnvalue_4) 1e+02))))