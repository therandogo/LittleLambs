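; Interactable component that lets its owner's static mesh be highlighted, picked up, carried and rotated for inspection.
; Hover toggles custom depth rendering on the mesh.
; Interaction grabs the mesh with a supplied physics handle and ignores Pawn collision until drop releases it and restores blocking.
; While held, Tick targets a point ahead of the camera and, during inspection, adds mouse delta to the target rotation.
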(event EventOnInteract
  (params (PhysicsHandler :type Physics%20Handle%20Component%20Object%20Reference) (CameraComponent :type Camera%20Component%20Object%20Reference))
  (CallFunction|OnInteraction PhysicsHandler CameraComponent))

(event EventTick
  (params (DeltaSeconds :type Float%20%28single-precision%29))
  (CallFunction|InspectionHandling))

(event EventHoveredCheck
  (params (IsHovered :type Boolean))
  (CallFunction|OnHoverRenderPass IsHovered))

(event EventBeginPlay
  (CallFunction|SetOwnerAttributes))

(event EventOnDrop
  (CallFunction|OnStopInteraction))

(event EventOnInspect
  (params (MouseDelta :type Vector%202D%20Structure))
  (Variables|MouseInput|SetMouse%20Delta MouseDelta)
  (Variables|ObjectState|SetInInspection true))

(event EventStopInspect
  (Variables|ObjectState|SetInInspection false))

(fn SetOwnerAttributes
  (bind _output_get (Variables|owner|SetOwnerActor (Components|GetOwner)))
  (Variables|Default|SetOwnerStaticMesh (Actor|GetComponentbyClass _output_get "/Script/Engine.StaticMeshComponent")))

(fn OnHoverRenderPass
  (params (bValue :type Boolean))
  (Rendering|SetRenderCustomDepth (Variables|Default|GetOwnerStaticMesh) bValue))

(fn OnInteraction
  (params (Physics%20Handler :type Physics%20Handle%20Component%20Object%20Reference) (Camera%20Component :type Camera%20Component%20Object%20Reference))
  (bind _ownerstaticmesh (Variables|Default|GetOwnerStaticMesh))
  (bind _ownerstaticmesh_2 (Variables|Default|GetOwnerStaticMesh))
  (Variables|Default|SetPhysics%20Handler Physics%20Handler)
  (Variables|Default|SetCamera%20Component Camera%20Component)
  (Physics|Components|PhysicsHandle|GrabComponentatLocationwithRotation (Variables|Default|GetPhysics%20Handler) _ownerstaticmesh_2 "None" (Transformation|GetWorldLocation _ownerstaticmesh) (Transformation|GetWorldRotation _ownerstaticmesh))
  (Collision|SetCollisionResponsetoChannel _ownerstaticmesh_2 "ECC_Pawn" "ECR_Ignore"))

(fn OnStopInteraction
  (Physics|Components|PhysicsHandle|ReleaseComponent (Variables|Default|GetPhysics%20Handler))
  (Variables|Default|SetPhysics%20Handler 0)
  (Variables|Default|SetCamera%20Component 0)
  (Collision|SetCollisionResponsetoChannel (Variables|Default|GetOwnerStaticMesh) "ECC_Pawn" "ECR_Block"))

(fn InspectionHandling
  (bind _mouse_delta (Variables|MouseInput|GetMouse%20Delta))
  (bind _camera_component (Variables|Default|GetCamera%20Component))
  (bind (_x _y) (Math|Vector2D|BreakVector2D _mouse_delta))
  (bind _physics_handler (Variables|Default|GetPhysics%20Handler)
    (:then
      (Physics|Components|PhysicsHandle|SetTargetLocation _physics_handler (+ (Transformation|GetWorldLocation _camera_component) (* (Math|Vector|GetForwardVector _camera_component) 2e+02)))
      (if (Variables|ObjectState|GetInInspection)
        (Class|PhysicsHandleComponent|SetTargetRotation _physics_handler (Math|Rotator|CombineRotators (.TargetRotation (Class|PhysicsHandleComponent|GetTargetLocationandRotation _physics_handler)) (Math|Rotator|MakeRotator 0.0 _y _x)))))
    (:else)))